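; Collectible pickup that updates the third-person character's item count and score when it enters the trigger area.
; A configured data table row sets the category, which adds points, does nothing (placebo) or subtracts points (poison).
; When the row is found, the pickup hides and disables its collision rather than being destroyed, then calls the character's end-game once the collected count equals its item limit.
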(event `self.TriggerArea.OnComponentBeginOverlap`
  (params (OverlappedComponent :type "PrimitiveComponent Object Reference") (OtherActor :type "Actor Object Reference") (OtherComp :type "PrimitiveComponent Object Reference") (OtherBodyIndex :type Integer) (bFromSweep :type Boolean) (SweepResult :type "HitResult Structure (by ref)"))
  (bind (_configoggetto_datatable _configoggetto_rowname) (break `DataTableRowHandle` (`self.ConfigOggetto`)))
  (bind _asbp_third_person_character (cast `/Game/ThirdPerson/Blueprints/BP_ThirdPersonCharacter` OtherActor))
  (set `/Game/ThirdPerson/Blueprints/BP_ThirdPersonCharacter.OggettiRaccolti` (+ (`/Game/ThirdPerson/Blueprints/BP_ThirdPersonCharacter.OggettiRaccolti` _asbp_third_person_character) 1) _asbp_third_person_character)
  (bind _returnvalue (`|GetDataTableRow` _configoggetto_datatable _configoggetto_rowname)
    (:`then`
      (bind (_categoria _valorepunti) (break `/Game/Consegna/BP/S_ItemData` _returnvalue))
      (switch `/Game/Consegna/BP/E_ItemCategory` _categoria
        (:`NewEnumerator0`
          (set `/Game/ThirdPerson/Blueprints/BP_ThirdPersonCharacter.PuntiTotali` (+ (`/Game/ThirdPerson/Blueprints/BP_ThirdPersonCharacter.PuntiTotali` _asbp_third_person_character) _valorepunti) _asbp_third_person_character))
        (:`NewEnumerator1`
          _)
        (:`NewEnumerator2`
          (set `/Game/ThirdPerson/Blueprints/BP_ThirdPersonCharacter.PuntiTotali` (- (`/Game/ThirdPerson/Blueprints/BP_ThirdPersonCharacter.PuntiTotali` _asbp_third_person_character) _valorepunti) _asbp_third_person_character)))
      (`self.SetActorHiddenInGame` true)
      (`self.SetActorEnableCollision` false)
      (if (== (`/Game/ThirdPerson/Blueprints/BP_ThirdPersonCharacter.OggettiRaccolti` _asbp_third_person_character) (`/Game/ThirdPerson/Blueprints/BP_ThirdPersonCharacter.LimiteOggetti` _asbp_third_person_character))
        (`/Game/ThirdPerson/Blueprints/BP_ThirdPersonCharacter.ActivateEndGame` _asbp_third_person_character)))))

(fn `UserConstructionScript`)